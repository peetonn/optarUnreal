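; AR pawn that starts an AR session with a debug menu and feeds device data to the Optar library.
; Each tick, it passes the camera texture to the OptarWorker, stores the keypoint count and publishes the device pose.
; On touch, it line-traces world objects first; only on a miss does it trace AR tracked geometry and spawn BP_Placeable there.
; Touch outcomes, including misses, are reported through ARHitResult.
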(event EventBeginPlay
  (Class|ARBlueprintLibrary|StartARSession "/Game/Data/D_SessionConfig.D_SessionConfig")
  ;[1 1 1] add debug widget
  (bind _returnvalue (UserInterface|CreateWidget "/Game/Blueprints/UI/BP_DebugMenu.BP_DebugMenu_C" (Game|GetPlayerController 0)))
  (bind _output_get (Variables|Default|SetdebugMenu _returnvalue))
  (UserInterface|Viewport|AddtoViewport _output_get 0)
  ;[1 1 1] spawn OptarWorker
  (Variables|Default|SetoptarWorker (Class|OptarWorker|GetDefaultWorker))
  ;[1 1 1] print optar library version info
  (bind _returnvalue_2 (Class|OptarWorker|GetOptarVersion))
  (Development|PrintText (Utilities|Text|ToText(String) _returnvalue_2)))

(event EventTick
  (params (DeltaSeconds :type Float%20%28single-precision%29))
  (bind (_devicerotation _deviceposition) (Class|HeadMountedDisplayFunctionLibrary|GetOrientationandPosition))
  (bind _optarworker (Variables|Default|GetoptarWorker))
  (Utilities|FlowControl|Sequence
    (:then_0
      ;[1 1 1] run optar
      (bind _returnvalue (Class|ARBlueprintLibrary|GetARTexture "CameraImage"))
      (bind _nkeypoints (Class|OptarWorker|ProcessCameraImage _optarworker _returnvalue))
      (Variables|Default|SetnKeyPoints _nkeypoints))
    (:then_1
      (Class|OptarWorker|PublishArPose _optarworker (Math|Transform|MakeTransform _deviceposition _devicerotation)))))

(event Input|TouchEvents|InputTouch
  (params (Location :type Vector) (FingerIndex :type ETouchIndex%20Enum))
  (bind _returnvalue (Game|GetPlayerController 0))
  (bind (_locationx _locationy) (Class|PlayerController|GetInputTouchState _returnvalue "Touch1"))
  (bind _returnvalue_2 (Math|Vector2D|MakeVector2D _locationx _locationy))
  (:Pressed
    (bind (_outhits _returnvalue_3) (CallFunction|WorldHitTest _returnvalue_2))
    (if _returnvalue_3
      (Default|CallARHitResult (|BreakHit (Utilities|Array|Get(acopy) _outhits)))
      (else
        ;[1 1 1] place object only if we haven't hit
        (bind _returnvalue_4 (Class|ARBlueprintLibrary|LineTraceTrackedObjects _returnvalue_2 false false))
        (Math|Integer|CompareInt (Utilities|Array|Length _returnvalue_4)
          (:>
            (Default|CallARHitResult (Class|ARTraceResultLibrary|GetTrackedGeometry (Utilities|Array|Get(acopy) _returnvalue_4)))
            (Game|SpawnActorfromClass "/Game/Blueprints/BP_Placeable.BP_Placeable_C" (Class|ARTraceResultLibrary|GetLocaltoWorldTransform (Utilities|Array|Get(acopy) _returnvalue_4)) "Undefined" 0 0))
          (:==
            ;[1 1 1] nothing hit
            (Default|CallARHitResult :!label _label))
          (:<
            (goto _label)))))))

(fn ConstructionScript)

(fn WorldHitTest
  (params (ScreenPosition :type Vector%202D%20Structure%20%28by%20ref%29))
  (bind _returnvalue (Game|GetPlayerController 0))
  (bind (_worldposition _worlddirection) (Class|GameplayStatics|DeprojectScreentoWorld _returnvalue ScreenPosition))
  (bind (_outhits _returnvalue_2) (Class|KismetSystemLibrary|LineTraceMultiforObjects _worldposition (+ _worldposition (* _worlddirection 1e+03)) (Utilities|Array|MakeArray "ObjectTypeQuery1" "ObjectTypeQuery2" "ObjectTypeQuery3" "ObjectTypeQuery4" "ObjectTypeQuery5" "ObjectTypeQuery6") false 0 "None" true))
  (return _outhits _returnvalue_2))