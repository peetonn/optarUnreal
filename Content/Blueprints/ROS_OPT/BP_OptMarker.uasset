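; BP_OptMarker is a marker actor with a colored sphere and a text label, updated from ROS data to display that data's Id.
; On BeginPlay it gives the sphere a dynamic material instance and sets a default green, with functions to set or read the color, set the text and toggle visibility.
; Each Tick rotates the label to face the player camera.
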(event EventBeginPlay
  (bind _returnvalue (Rendering|Material|CreateDynamicMaterialInstance "/Engine/BasicShapes/BasicShapeMaterial.BasicShapeMaterial" "MarkerMat" "Transient" :!class /Script/Engine.KismetMaterialLibrary))
  (bind _output_get (Variables|Default|SetmarkerMatInstance _returnvalue))
  (Rendering|Material|SetMaterial (Variables|Default|GetSphere) 0 _output_get)
  (CallFunction|SetColor "(R=0.083612,G=0.922781,B=0.289628,A=1.000000)"))

(event Collision|EventActorBeginOverlap
  (params (OtherActor :type Actor%20Object%20Reference)))

(event EventTick
  (params (DeltaSeconds :type Float%20%28single-precision%29))
  (Transformation|SetWorldRotation (Variables|Default|GetTextRender) (Math|Rotator|FindLookatRotation (Transformation|GetActorLocation) (Camera|GetCameraLocation (Game|GetPlayerCameraManager 0))) false false))

(event EventUpdatefromRosData
  (params (rosData :type ROS%20Msg%20Track%20Object%20Reference))
  (CallFunction|SetMarkerText (Utilities|String|ToString(Integer) (Variables|/Script/OptMsgs.ROSMsgTrack|GetId rosData))))

(fn ConstructionScript)

(fn SetColor
  (params (markerColor :type Linear%20Color%20Structure))
  (Rendering|Material|SetVectorParameterValue (Variables|Default|GetmarkerMatInstance) "Color" markerColor :!class /Script/Engine.MaterialInstanceDynamic))

(fn GetColor
  (bind _returnvalue (Rendering|Material|GetVectorParameterValue (Variables|Default|GetmarkerMatInstance) "Color" :!class /Script/Engine.MaterialInstanceDynamic))
  (return _returnvalue))

(fn SetVisibility
  (params (isVisible :type Boolean))
  (Rendering|SetVisibility (Variables|Default|GetDefaultSceneRoot) isVisible true))

(fn SetMarkerText
  (params (text :type String))
  (Rendering|Components|TextRender|SetText (Variables|Default|GetTextRender) (Utilities|Text|ToText(String) text)))