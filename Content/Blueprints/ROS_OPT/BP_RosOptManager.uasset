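; Manager actor that subscribes to a ROS OPT people-tracking topic, optionally server-only, and shows each track as a marker actor.
; Each TrackArray message is diffed against active tracks by ID, firing added, updated and removed events.
; Its own handlers take markers from a growable hidden-actor pool, recycling them on removal.
; Markers are positioned by offsetting track positions from RosOrigin's location and receive data through BP_Interface_OptMarker.
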(event OnNewMessage(ROSTopic)
  (params (Message :type ROS%20Message%20Base%20Object%20Reference))
  (bind _asrosmsg_track_array (Utilities|Casting|CastToROSMsgTrackArray Message)
    (:then
      (OPTTracksHandling|UpdateTracks _asrosmsg_track_array))
    (:CastFailed
      (Class|DDBlueprintLibrary|LogWarning "Failed to cast message to OPT/TrackArray "))))

(event EventBeginPlay
  (bind _rostopic (Variables|Default|GetROSTopic))
  (Utilities|FlowControl|Sequence
    (:then_0
      (if (Variables|Default|GetserverOnly)
        (if (Networking|IsServer)
          (Utilities|IsValid (Variables|ROS|GetrosOrigin) :!label _label
            (:Is%20Valid
              (Development|PrintString "Initializing ROS topic subscriber...")
              (Class|ROSTopic|Initialize _rostopic (Variables|ROS|GetoptPeopleTracksTopic) "/Script/OptMsgs.ROSMsgTrackArray")
              (Class|ROSTopic|Subscribe _rostopic))
            (:Is%20Not%20Valid
              (Class|DDBlueprintLibrary|LogError "ROS Origin must be set up"))))
        (else
          (goto _label))))
    (:then_1
      (MarkerPool|AllocateMarkerPool 32))
    (:then_2
      (EventDispatchers|BindEventtoOptTrackAdded (EventDispatchers|CreateEvent :!event OnNewOptTrackAdded))
      (EventDispatchers|BindEventtoOptTrackRemoved (EventDispatchers|CreateEvent :!event OnOptTrackRemoved))
      (EventDispatchers|BindEventtoOptTrackUpdated (EventDispatchers|CreateEvent :!event OnOptTrackUpdated)))))

(event Collision|EventActorBeginOverlap
  (params (OtherActor :type Actor%20Object%20Reference)))

(event EventTick
  (params (DeltaSeconds :type Float%20%28single-precision%29)))

(fn ConstructionScript)

(fn UpdateTracks
  (params (trackArrayMsg :type ROS%20Msg%20Track%20Array%20Object%20Reference))
  (bind _activetracks (Variables|Default|GetactiveTracks))
  (bind _keys (Utilities|Map|Keys (Variables|Default|GetactiveTracks)))
  (Utilities|Set|AddItems (LocalVariables|GetcurrentTracks) _keys)
  (Utilities|FlowControl|Sequence
    (:then_1
      (for _array_element (Variables|/Script/OptMsgs.ROSMsgTrackArray|GetTracks trackArrayMsg)
        (if (Utilities|Set|Contains (LocalVariables|GetcurrentTracks) (Variables|/Script/OptMsgs.ROSMsgTrack|GetId _array_element))
          (Utilities|Set|Remove (LocalVariables|GetcurrentTracks) (Variables|/Script/OptMsgs.ROSMsgTrack|GetId _array_element))
          (Utilities|Set|Add (LocalVariables|GetupdatedTracks) (Variables|/Script/OptMsgs.ROSMsgTrack|GetId _array_element))
          (else
            (Utilities|Set|Add (LocalVariables|GetnewTracks) (Variables|/Script/OptMsgs.ROSMsgTrack|GetId _array_element))))
        (Utilities|Map|Add (Variables|Default|GetactiveTracks) (Variables|/Script/OptMsgs.ROSMsgTrack|GetId _array_element) _array_element))
      (Utilities|FlowControl|Sequence
        (:then_0
          ;[1 0 0.07571] track left
          (bind _result (Utilities|Set|ToArray (LocalVariables|GetcurrentTracks)))
          (for _array_element_2 _result
            (Default|CallOptTrackRemoved (.Value (Utilities|Map|Find _activetracks _array_element_2)))
            (Utilities|Map|Remove _activetracks _array_element_2)))
        (:then_1
          ;[0.1447 0.4846 1] track updated
          (bind _result_2 (Utilities|Set|ToArray (LocalVariables|GetupdatedTracks)))
          (for _array_element_3 _result_2
            (Default|CallOptTrackUpdated (.Value (Utilities|Map|Find (Variables|Default|GetactiveTracks) _array_element_3)))))
        (:then_2
          ;[0.000982 1 0.1819] track entered
          (bind _result_3 (Utilities|Set|ToArray (LocalVariables|GetnewTracks)))
          (for _array_element_4 _result_3
            (Default|CallOptTrackAdded (.Value (Utilities|Map|Find (Variables|Default|GetactiveTracks) _array_element_4)))))))))

(fn OnNewOptTrackAdded
  (params (trackMsg :type ROS%20Msg%20Track%20Object%20Reference))
  (bind _output_get (LocalVariables|SetnewMarker (MarkerPool|GetMarker)))
  (OPTTracksHandling|UpdateMarkerfromROSData _output_get trackMsg)
  (Utilities|Map|Add (Variables|Default|GetactiveMarkers) (Variables|/Script/OptMsgs.ROSMsgTrack|GetId trackMsg) (LocalVariables|GetnewMarker)))

(fn OnOptTrackRemoved
  (params (trackMsg :type ROS%20Msg%20Track%20Object%20Reference))
  (bind _id (Variables|/Script/OptMsgs.ROSMsgTrack|GetId trackMsg))
  (bind _activemarkers (Variables|Default|GetactiveMarkers))
  (MarkerPool|RecycleMarker (.Value (Utilities|Map|Find _activemarkers _id)))
  (Utilities|Map|Remove _activemarkers _id))

(fn OnOptTrackUpdated
  (params (trackMsg :type ROS%20Msg%20Track%20Object%20Reference))
  (OPTTracksHandling|UpdateMarkerfromROSData (.Value (Utilities|Map|Find (Variables|Default|GetactiveMarkers) (Variables|/Script/OptMsgs.ROSMsgTrack|GetId trackMsg))) trackMsg))

(fn AllocateMarkerPool
  (params (n :type Integer))
  (for _index (range 1 n)
    (bind _returnvalue (Game|SpawnActorfromClass (Variables|ROS|GetoptMarkerClass) (Transformation|GetActorTransform (Variables|ROS|GetrosOrigin)) "AlwaysSpawn" self 0))
    (MarkerPool|RecycleMarker _returnvalue)))

(fn GetMarker
  (bind _markerspool (Variables|MarkerPool|GetmarkersPool))
  (if (== (Utilities|Array|Length (Variables|MarkerPool|GetmarkersPool)) 0)
    (MarkerPool|AllocateMarkerPool 16))
  (bind _output_get (LocalVariables|SetnewMarker (Utilities|Array|Get(acopy) _markerspool)))
  (Utilities|Array|RemoveItem _markerspool _output_get)
  (Rendering|SetActorHiddenInGame (LocalVariables|GetnewMarker) false)
  (Transformation|SetActorTransform (LocalVariables|GetnewMarker) (Transformation|GetActorTransform (Variables|ROS|GetrosOrigin)))
  (return (LocalVariables|GetnewMarker)))

(fn RecycleMarker
  (params (marker :type Actor%20Object%20Reference))
  (Rendering|SetActorHiddenInGame marker true)
  (Utilities|Array|Add (Variables|MarkerPool|GetmarkersPool) marker))

(fn UpdateMarkerfromROSData
  (params (marker :type Actor%20Object%20Reference) (rosData :type ROS%20Msg%20Track%20Object%20Reference))
  (Utilities|FlowControl|Sequence
    (:then_0
      (Transformation|SetActorLocation marker (+ (Class|ROSMsgTrack|GetPositionasVector rosData) (Transformation|GetActorLocation (Variables|ROS|GetrosOrigin))) false false))
    (:then_1
      (bind _asbp_interface_opt_marker (Utilities|Casting|CastToBP_Interface_OptMarker marker))
      (Default|UpdatefromRosData _asbp_interface_opt_marker rosData))))