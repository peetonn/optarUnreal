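; WolfCub_BP is a wolf cub animal Blueprint that stops moving while it sits or eats.
; Each Tick, the IsSitting or IsEating flags zero the CharacterMovement walk speed and clear CanMove.
; When neither flag is set, a short Delay passes before CanMove and the walk speed are restored.
; The construction script only calls its parent.
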(event EventBeginPlay)

(event Collision|EventActorBeginOverlap
  (params (OtherActor :type Actor%20Object%20Reference)))

(event EventTick
  (params (DeltaSeconds :type Float%20%28single-precision%29))
  (if (or (Variables|Default|GetIsSitting) (Variables|Default|GetIsEating))
    (Variables|/Script/Engine.CharacterMovementComponent|SetMaxWalkSpeed (Variables|Character|GetCharacterMovement) 0.0)
    (Variables|Default|SetCanMove false)
    (elif (not (Variables|Default|GetCanMove))
      (Utilities|FlowControl|Delay 1.5)
      (Variables|Default|SetCanMove true)
      (Variables|/Script/Engine.CharacterMovementComponent|SetMaxWalkSpeed (Variables|Character|GetCharacterMovement) 1.5e+02))))

(fn ConstructionScript
  (|CallParentFunction))