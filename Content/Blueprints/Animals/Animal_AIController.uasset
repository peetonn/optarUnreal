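; AI controller for animals that runs the Animal behavior tree on BeginPlay.
; AI perception updates store a sensed BP_OptMarker actor in the FriendPlayer blackboard key.
; When the marker is no longer sensed, it clears that key and calls SetFocus with no actor.
; A branch that would treat BP_VRPawn as the friend player is present but disconnected.
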(event OnTargetPerceptionUpdated(AIPerception)
  (params (Actor :type Actor%20Object%20Reference) (Stimulus :type AI%20Stimulus%20Structure))
  (bind _returnvalue (AI|GetBlackboard 0))
  (bind _returnvalue_2 (Utilities|Name|MakeLiteralName "FriendPlayer"))
  (bind _asbp_opt_marker (Utilities|Casting|CastToBP_OptMarker Actor))
  (if (.bSuccessfullySensed (Utilities|Struct|BreakAIStimulus Stimulus))
    (AI|Components|Blackboard|SetValueasObject _returnvalue _returnvalue_2 _asbp_opt_marker)
    (else
      (AI|Components|Blackboard|SetValueasObject _returnvalue _returnvalue_2 0)
      (AI|SetFocus))))

(event EventBeginPlay
  (AI|RunBehaviorTree "/Game/AI/Animal_BehaviorTree.Animal_BehaviorTree"))

(fn ConstructionScript)