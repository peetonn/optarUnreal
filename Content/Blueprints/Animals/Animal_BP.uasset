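; Animal Blueprint with character movement that tracks hunger and sitting state.
; Tick clears the sitting flag once movement speed exceeds a small threshold.
; HungerLevel works as a fullness value: IncreaseHunger lowers it by a step scaled by HungerMultiplier, without clamping, and ResetHunger restores it to full.
; Nothing in this graph calls the hunger events or sets the sitting flag to true.
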(event Custom|IncreaseHunger
  (Variables|Default|SetHungerLevel (- (Variables|Default|GetHungerLevel) (* 0.1 (Variables|Default|GetHungerMultiplier)))))

(event Custom|ResetHunger
  (Variables|Default|SetHungerLevel 1.0))

(event EventTick
  (params (DeltaSeconds :type Float%20%28single-precision%29))
  (if (and (Variables|Default|GetIsSitting) (> (Math|Vector|VectorLength (Variables|/Script/Engine.MovementComponent|GetVelocity (Variables|Character|GetCharacterMovement))) 1e+01))
    (Variables|Default|SetIsSitting false)))

(fn ConstructionScript)