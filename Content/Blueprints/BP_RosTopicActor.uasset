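; An actor that mirrors a ROS pose topic, moving itself to match each received pose.
; On BeginPlay its ROSTopic component subscribes to the turtle1 pose topic using the ROSMsgPose message class.
; Each new message is cast to a pose, whose position and orientation set the actor transform at unit scale, without sweep or unit conversion in the graph.
; The applied transform, or a cast failure, is printed for debugging.
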(event OnNewMessage(ROSTopic)
  (params (Message :type ROS%20Message%20Base%20Object%20Reference))
  (bind _asrosmsg_pose (Utilities|Casting|CastToROSMsgPose Message)
    (:then
      (Transformation|SetActorTransform self (Math|Transform|MakeTransform (Class|ROSMsgPose|PositionasFVector _asrosmsg_pose) (Class|KismetMathLibrary|QuatRotator (Class|ROSMsgPose|OrientationasQuad _asrosmsg_pose))))
      (Development|PrintString (Utilities|String|ToString(Text) (Utilities|Text|FormatText "Set transform {t}" (Utilities|Text|ToText(String) (Math|Transform|MakeTransform (Class|ROSMsgPose|PositionasFVector _asrosmsg_pose) (Class|KismetMathLibrary|QuatRotator (Class|ROSMsgPose|OrientationasQuad _asrosmsg_pose))))))))
    (:CastFailed
      (Development|PrintString "FAILED TO CAST MESSAGE TO POSE "))))

(event EventBeginPlay
  (bind _rostopic (Variables|Default|GetROSTopic))
  (Class|ROSTopic|Initialize _rostopic "/turtle1/pose" "/Script/Rosbridge2Unreal.ROSMsgPose")
  (Class|ROSTopic|Subscribe _rostopic))

(event Collision|EventActorBeginOverlap
  (params (OtherActor :type Actor%20Object%20Reference)))

(event EventTick
  (params (DeltaSeconds :type Float%20%28single-precision%29)))

(fn ConstructionScript)