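; BP_ARGameMode is a game mode that owns the loading and saving of a BP_OptarSaveGame object.
; On PostLogin it loads the default slot into its SaveGame variable, constructing a fresh save object if the load or cast yields nothing valid.
; A SaveGame event writes that object back to the same slot, but nothing in this Blueprint calls it.
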(event Custom|Load%20Saved%20Game
  ;[1 1 1] load / save game
  (bind _returnvalue (SaveGame|LoadGamefromSlot (Variables|Default|GetdefaultSaveSlot)))
  (bind _asbp_optar_save_game (Utilities|Casting|CastToBP_OptarSaveGame _returnvalue)
    (:then
      (Utilities|IsValid _asbp_optar_save_game
        (:Is%20Valid
          (Variables|Default|SetsaveGame _asbp_optar_save_game))
        (:Is%20Not%20Valid
          (bind _returnvalue_2 (Game|ConstructObjectfromClass "/Game/Blueprints/BP_OptarSaveGame.BP_OptarSaveGame_C" self :!label _label))
          (Variables|Default|SetsaveGame _returnvalue_2))))
    (:CastFailed
      (goto _label))))

(event Custom|Save%20Game
  ;[1 1 1] load / save game
  (SaveGame|SaveGametoSlot (Variables|Default|GetsaveGame) (Variables|Default|GetdefaultSaveSlot)))

(event EventBeginPlay)

(event EventTick
  (params (DeltaSeconds :type Float%20%28single-precision%29)))

(event EventPostLogin
  (params (NewPlayer :type Player%20Controller%20Object%20Reference))
  (CallFunction|LoadSavedGame))

(fn ConstructionScript)