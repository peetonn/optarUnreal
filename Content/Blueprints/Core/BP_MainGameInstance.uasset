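; BP_MainGameInstance is the game instance that owns the persistent save object and handles connecting to a server.
; On Init it loads BP_OptarSaveGame from its slot, or constructs and saves a new one if the load or cast fails.
; ConnectToServer stores the IP and runs an "open" console command, passing the client platform name as a URL option.
; Loading and connecting log their progress, and a failed save logs an error.
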(event EventInit
  (CallFunction|LoadGame))

(fn ConnecttoServer
  (params (ip :type String))
  (bind _output_get (LocalVariables|SetipAddress ip))
  (Class|DDBlueprintLibrary|LogInfo (Utilities|String|ToString(Text) (Utilities|Text|FormatText "Connecting to {ip}..." _output_get)))
  (Development|ExecuteConsoleCommand (Utilities|String|ToString(Text) (Utilities|Text|FormatText "open {serverIp}?ClientPlatform={clientPlatform}" (Utilities|Text|ToText(String) (LocalVariables|GetipAddress)) (Utilities|Text|ToText(String) (Game|GetPlatformName)))) 0))

(fn SaveGame
  (bind _returnvalue (SaveGame|SaveGametoSlot (Variables|SaveGame|GetsaveGame) (Variables|SaveGame|GetsaveGameSlot)))
  (if (not _returnvalue)
    (Class|DDBlueprintLibrary|LogError "Error saving the game")))

(fn LoadGame
  (bind _returnvalue (SaveGame|LoadGamefromSlot (Variables|SaveGame|GetsaveGameSlot)))
  (bind _asbp_optar_save_game (Utilities|Casting|CastToBP_OptarSaveGame _returnvalue)
    (:then
      (Variables|SaveGame|SetsaveGame _asbp_optar_save_game)
      (Class|DDBlueprintLibrary|LogInfo "Loaded game"))
    (:CastFailed
      (bind _returnvalue_2 (Game|ConstructObjectfromClass "/Game/Blueprints/BP_OptarSaveGame.BP_OptarSaveGame_C" self))
      (Variables|SaveGame|SetsaveGame _returnvalue_2)
      (CallFunction|SaveGame))))