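; Component for player controllers that owns the debug menu and toggles it on screen.
; On BeginPlay it creates a BP_DebugMenu widget and binds its close event to hide the menu.
; SetMenuVisibility adds or removes the widget, switching the owning BasePlayerController between UI-only and game-only input and toggling the mouse cursor.
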(event Custom|Close%20Menu
  (CallFunction|SetMenuVisibility false))

(event EventBeginPlay
  (bind _returnvalue (Game|ConstructObjectfromClass "/Game/Blueprints/UI/BP_DebugMenu.BP_DebugMenu_C" self))
  (bind _output_get (Variables|Menu|SetuiWidget _returnvalue))
  (EventDispatchers|BindEventtoOnCloseMenu _output_get (delegate Custom|Close%20Menu)))

(event EventTick
  (params (DeltaSeconds :type Float%20%28single-precision%29)))

(fn SetMenuVisibility
  (params (isMenuVisible :type Boolean))
  (bind _newparam (CallFunction|GetMyOwner))
  (bind _uiwidget (Variables|Menu|GetuiWidget))
  (bind _output_get (Variables|Menu|SetisMenuVisible isMenuVisible))
  (if _output_get
    (UserInterface|Viewport|AddtoViewport _uiwidget 0)
    (Input|SetInputModeUIOnly _newparam (Variables|Menu|GetuiWidget) "DoNotLock")
    (Variables|/Script/Engine.PlayerController|SetbShowMouseCursor _newparam true)
    (else
      (Widget|RemovefromParent _uiwidget)
      (Input|SetInputModeGameOnly _newparam)
      (Variables|/Script/Engine.PlayerController|SetbShowMouseCursor _newparam false)))
  (return))

(fn GetMyOwner
  (bind _asbase_player_controller (Utilities|Casting|CastToBasePlayerController (Components|GetOwner)))
  (return _asbase_player_controller))