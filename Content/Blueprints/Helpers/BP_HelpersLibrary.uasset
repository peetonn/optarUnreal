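; Blueprint function library of shared helpers for an AR game, giving quick access to core gameplay objects.
; It wraps the AR support check and returns the game instance, player 0's AR pawn and AR controller, each cast to its project class.
; The pawn and controller getters log a warning when their cast fails, while the game instance getter does not.
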(fn IsARCapablePlatform
  (bind _returnvalue (Class|ARBlueprintLibrary|IsARSupported))
  (return _returnvalue))

(fn GetMyGameInstance
  (bind _asbp_main_game_instance (Utilities|Casting|CastToBP_MainGameInstance (Game|GetGameInstance)))
  (return _asbp_main_game_instance))

(fn GetMyARPawn
  (bind _asbp_arpawn (Utilities|Casting|CastToBP_ARPawn (Pawn|GetControlledPawn (Game|GetPlayerController 0)))
    (:then
      (return _asbp_arpawn))
    (:CastFailed
      (Class|DDBlueprintLibrary|LogWarning "Failed to cast pawn to ARPawn")
      (return 0))))

(fn GetMyARPlayerController
  (bind _asbp_arcontroller (Utilities|Casting|CastToBP_ARController (Game|GetPlayerController 0))
    (:then
      (return _asbp_arcontroller))
    (:CastFailed
      (Class|DDBlueprintLibrary|LogWarning "Failed to cast controller to ARController")
      (return 0))))